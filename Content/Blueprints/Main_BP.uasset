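; Main_BP is the player character, switching between Dash, Fury, Tank and Ranged styles and sliding on ice.
; Number keys swap the skeletal mesh and add that style's widget, gated by Frozen and, except Dash, unlock flags; E auto-equips each unlocked style once through DoOnce.
; A looping timer reads the floor's surface type to set friction, braking and acceleration.
; MyGhostTrails spawns a trail actor at the mesh; a delayed triple-spawn chain is unconnected.
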(event Custom|SetGroundFriction
  (bind _charactermovement (Variables|Character|GetCharacterMovement))
  (bind _charactermovement_2 (Variables|Character|GetCharacterMovement))
  (bind _currentfloor (Variables|/Script/Engine.CharacterMovementComponent|GetCurrentFloor _charactermovement))
  (bind _returnvalue (Collision|GetSurfaceType (.hitresult _currentfloor)))
  (Variables|/Script/Engine.CharacterMovementComponent|SetGroundFriction _charactermovement_2 (Utilities|Select :Index _returnvalue :SurfaceType_Default 8.0 :SurfaceType1 0.2))
  (Variables|/Script/Engine.CharacterMovementComponent|SetBrakingDecelerationWalking _charactermovement_2 (Utilities|Select :Index _returnvalue :SurfaceType_Default 2048.0 :SurfaceType1 2e+02))
  (Variables|/Script/Engine.CharacterMovementComponent|SetMaxAcceleration _charactermovement_2 (Utilities|Select :Index _returnvalue :SurfaceType_Default 2048.0 :SurfaceType1 2e+02)))

(event Custom|MyGhostTrails
  (Game|SpawnActorfromClass "/Game/Blueprints/GhostTrails_BP.GhostTrails_BP_C" (Transformation|GetWorldTransform (Variables|Character|GetMesh)) "Undefined" 0 0))

(event Collision|EventActorBeginOverlap
  (params (OtherActor :type Actor%20Object%20Reference)))

(event EventTick
  (params (DeltaSeconds :type Float%20%28single-precision%29)))

(event EventBeginPlay
  (bind _returnvalue (Utilities|Time|SetTimerbyFunctionName 0 "SetGroundFriction" 0.1 true))
  (Variables|Default|SetGround%20Friction _returnvalue))

(event Input|KeyboardEvents|1
  (params (Key :type Key%20Structure :default "None"))
  (:Pressed
    (if (not (Variables|Default|GetFrozen))
      (Class|SkinnedMeshComponent|SetSkeletalMesh (Variables|Character|GetMesh) "/Game/Meshes/AlterMC/Main_Character_Dash_001.Main_Character_Dash_001" true)
      (bind _returnvalue (UserInterface|CreateWidget "/Game/Menus/HUD/Dash_Widget.Dash_Widget_C"))
      (UserInterface|Viewport|AddtoViewport _returnvalue 0))))

(event Input|KeyboardEvents|2
  (params (Key :type Key%20Structure :default "None"))
  (:Pressed
    (if (not (Variables|Default|GetFrozen))
      (if (Variables|Default|GetbFuryUnlocked)
        (Class|SkinnedMeshComponent|SetSkeletalMesh (Variables|Character|GetMesh) "/Game/Meshes/AlterMC/Main_Character_Fury_001.Main_Character_Fury_001" true)
        (bind _returnvalue (UserInterface|CreateWidget "/Game/Menus/HUD/Fury_Widget.Fury_Widget_C"))
        (UserInterface|Viewport|AddtoViewport _returnvalue 0)))))

(event Input|KeyboardEvents|E
  (params (Key :type Key%20Structure :default "None"))
  (:Pressed
    (if (not (Variables|Default|GetFrozen))
      (if (Variables|Default|GetbRangedUnlocked)
        (Utilities|FlowControl|DoOnce false
          (:Completed
            (Class|SkinnedMeshComponent|SetSkeletalMesh (Variables|Character|GetMesh) "/Game/Meshes/AlterMC/Main_Character_Range_001.Main_Character_Range_001" true)
            (bind _returnvalue (UserInterface|CreateWidget "/Game/Menus/HUD/Ranged_Widget.Ranged_Widget_C"))
            (UserInterface|Viewport|AddtoViewport _returnvalue 0)))))))

(event Input|KeyboardEvents|3
  (params (Key :type Key%20Structure :default "None"))
  (:Pressed
    (if (not (Variables|Default|GetFrozen))
      (if (Variables|Default|GetbDefenceUnlocked)
        (Class|SkinnedMeshComponent|SetSkeletalMesh (Variables|Character|GetMesh) "/Game/Meshes/AlterMC/Main_Character_Tank_001.Main_Character_Tank_001" true)
        (bind _returnvalue (UserInterface|CreateWidget "/Game/Menus/HUD/Tank_Widget.Tank_Widget_C"))
        (UserInterface|Viewport|AddtoViewport _returnvalue 0)))))

(event Input|KeyboardEvents|E
  (params (Key :type Key%20Structure :default "None"))
  (:Pressed
    (if (not (Variables|Default|GetFrozen))
      (if (Variables|Default|GetbFuryUnlocked)
        (Utilities|FlowControl|DoOnce false
          (:Completed
            (Class|SkinnedMeshComponent|SetSkeletalMesh (Variables|Character|GetMesh) "/Game/Meshes/AlterMC/Main_Character_Fury_001.Main_Character_Fury_001" true)
            (bind _returnvalue (UserInterface|CreateWidget "/Game/Menus/HUD/Fury_Widget.Fury_Widget_C"))
            (UserInterface|Viewport|AddtoViewport _returnvalue 0)))))))

(event Input|KeyboardEvents|4
  (params (Key :type Key%20Structure :default "None"))
  (:Pressed
    (if (not (Variables|Default|GetFrozen))
      (if (Variables|Default|GetbRangedUnlocked)
        (Class|SkinnedMeshComponent|SetSkeletalMesh (Variables|Character|GetMesh) "/Game/Meshes/AlterMC/Main_Character_Range_001.Main_Character_Range_001" true)
        (bind _returnvalue (UserInterface|CreateWidget "/Game/Menus/HUD/Ranged_Widget.Ranged_Widget_C"))
        (UserInterface|Viewport|AddtoViewport _returnvalue 0)))))

(event Input|KeyboardEvents|E
  (params (Key :type Key%20Structure :default "None"))
  (:Pressed
    (if (not (Variables|Default|GetFrozen))
      (if (Variables|Default|GetbDefenceUnlocked)
        (Utilities|FlowControl|DoOnce false
          (:Completed
            (Class|SkinnedMeshComponent|SetSkeletalMesh (Variables|Character|GetMesh) "/Game/Meshes/AlterMC/Main_Character_Tank_001.Main_Character_Tank_001" true)
            (bind _returnvalue (UserInterface|CreateWidget "/Game/Menus/HUD/Tank_Widget.Tank_Widget_C"))
            (UserInterface|Viewport|AddtoViewport _returnvalue 0)))))))

(event Input|MouseEvents|RightMouseButton
  (params (Key :type Key%20Structure :default "None")))

(fn ConstructionScript)